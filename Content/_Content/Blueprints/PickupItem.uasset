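; Pickup actor that restores either ammo or health to the first-person character that overlaps it, then destroys itself.
; The Type enum selects the effect, resetting that PlayerInfoComponent value to its class default rather than adding an amount.
; The construction script shows the matching visual component, hides the other and stores it as CurrentVisual.
; Tick makes that visual bob on a sine wave and spin around its vertical axis.
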(event EventBeginPlay)

(event Collision|EventActorBeginOverlap
  (params (OtherActor :type Actor%20Object%20Reference))
  (bind (_health _currentammo) (Utilities|GetClassDefaults "/Game/_Content/Blueprints/PlayerInfoComponent.PlayerInfoComponent_C"))
  (bind _asbp_first_person_character (Utilities|Casting|CastToBP_FirstPersonCharacter OtherActor))
  (switch Utilities|FlowControl|Switch|SwitchonPickupType (Variables|Default|GetType)
    (:NewEnumerator0
      (Variables|/Game/_Content/Blueprints/PlayerInfoComponent.PlayerInfoComponent_C|SetCurrentAmmo (Variables|/Game/FirstPerson/Blueprints/BP_FirstPersonCharacter.BP_FirstPersonCharacter_C|GetPlayerInfoComponent _asbp_first_person_character) _currentammo))
    (:NewEnumerator1
      (Variables|/Game/_Content/Blueprints/PlayerInfoComponent.PlayerInfoComponent_C|SetHealth (Variables|/Game/FirstPerson/Blueprints/BP_FirstPersonCharacter.BP_FirstPersonCharacter_C|GetPlayerInfoComponent _asbp_first_person_character) _health)))
  (Actor|DestroyActor))

(event EventTick
  (params (DeltaSeconds :type Float%20%28single-precision%29))
  (bind _currentvisual (Variables|Default|GetCurrentVisual))
  (Transformation|SetRelativeLocation _currentvisual (Math|Vector|MakeVector 0.0 0.0 (* (Math|Trig|Sin(Radians) (* (Utilities|Time|GetRealTimeSeconds) 5.0)) 4.0)) false false)
  (Transformation|AddRelativeRotation _currentvisual (Math|Rotator|MakeRotator 0.0 0.0 (* DeltaSeconds 4e+01)) false false))

(fn ConstructionScript
  (bind _health (Variables|Default|GetHealth))
  (bind _ammo (Variables|Default|GetAmmo))
  (switch Utilities|FlowControl|Switch|SwitchonPickupType (Variables|Default|GetType)
    (:NewEnumerator0
      (Rendering|SetVisibility _ammo true false)
      (Rendering|SetVisibility _health false false)
      (Variables|Default|SetCurrentVisual _ammo))
    (:NewEnumerator1
      (Rendering|SetVisibility _ammo false false)
      (Rendering|SetVisibility _health true false)
      (Variables|Default|SetCurrentVisual _health))))