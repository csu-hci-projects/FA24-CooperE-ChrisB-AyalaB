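; Zombie enemy that moves along a timeline track and can be destroyed by first-person projectiles.
; A timeline started on BeginPlay sets the Zombie component's relative location, with a delay in its update toggling IsLooped to alternate play and reverse.
; Projectile hits destroy it if Health is at most 50, incrementing the player's PlayerInfoComponent destroyed-target count.
; Otherwise, Health becomes 50 minus Health, so the subtraction is inverted.
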(event EventBeginPlay
  (bind _newtrack_1 (Timeline|Moving Play)
    (:Update
      (Transformation|SetRelativeLocation (Variables|Default|Getzombie) _newtrack_1 false false)
      (Utilities|FlowControl|Delay 3.0)
      (if (Variables|Default|GetisLooped)
        (Variables|Default|SetisLooped false)
        (Timeline|Moving Reverse)
        (else
          (Variables|Default|SetisLooped true)
          (Timeline|Moving Play))))))

(event Collision|EventHit
  (params (MyComp :type Primitive%20Component%20Object%20Reference) (Other :type Actor%20Object%20Reference) (OtherComp :type Primitive%20Component%20Object%20Reference) (bSelfMoved :type Boolean) (HitLocation :type Vector :default "0, 0, 0") (HitNormal :type Vector :default "0, 0, 0") (NormalImpulse :type Vector :default "0, 0, 0") (Hit :type Hit%20Result%20Structure%20%28by%20ref%29))
  (Utilities|Casting|CastToBP_FirstPersonProjectile Other)
  (if (<= 0 (- 50 (Variables|Default|Gethealth)))
    (bind _asbp_first_person_character (Utilities|Casting|CastToBP_FirstPersonCharacter (Game|GetPlayerCharacter 0)))
    (Variables|/Game/_Content/Blueprints/PlayerInfoComponent.PlayerInfoComponent_C|SetnumTargetsDestroyed (Actor|GetComponentbyClass _asbp_first_person_character "/Game/_Content/Blueprints/PlayerInfoComponent.PlayerInfoComponent_C") (- (Variables|/Game/_Content/Blueprints/PlayerInfoComponent.PlayerInfoComponent_C|GetnumTargetsDestroyed (Actor|GetComponentbyClass _asbp_first_person_character "/Game/_Content/Blueprints/PlayerInfoComponent.PlayerInfoComponent_C")) -1))
    (Actor|DestroyActor)
    (else
      (Variables|Default|Sethealth (- 50 (Variables|Default|Gethealth))))))

(fn ConstructionScript)